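; Flag zombie Blueprint, a zombie variant that drives its own animation Blueprint from its death and eating states.
; On BeginPlay it casts the animation component's instance to FlagZombieAnimBP and caches it.
; The die and eat event overrides call their parent versions, then copy the IsDie and IsEat flags into that anim instance.
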(event `self.ReceiveBeginPlay`
  (bind _asflag_zombie_anim_bp (cast `/Game/BP/Zombies/FlagZombie/FlagZombieAnimBP` (`PaperZDAnimationComponent.AnimInstance` (`self.AnimationComponent`))))
  (set `self.AnimBP` _asflag_zombie_anim_bp))

(event `self.ReceiveTick`
  (params (DeltaSeconds :type "Float (single-precision)")))

(event `self.OnZombiesDie`
  (params (IsDie :type Boolean))
  (`parent.OnZombiesDie` IsDie)
  (set `/Game/BP/Zombies/FlagZombie/FlagZombieAnimBP.IsDie` IsDie (`self.AnimBP`)))

(event `self.OnZombiesEat`
  (params (IsEat :type Boolean))
  (`parent.OnZombiesEat` IsEat)
  (set `/Game/BP/Zombies/FlagZombie/FlagZombieAnimBP.IsEat` IsEat (`self.AnimBP`)))

(fn `UserConstructionScript`)